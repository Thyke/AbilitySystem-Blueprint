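; GA_Jump is a gameplay ability that makes the instigating Character jump and stays active until it lands.
; On activation it runs the parent logic, casts and stores the instigator as a Character, calls Jump and binds to its Landed delegate.
; The landed callback calls EndAbility, which runs the parent end logic and unbinds the delegate.
; A failed Character cast stops activation without ending the ability.
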(event `self.ActivateAbility`
  (params (Instigator :type "Actor Object Reference"))
  (`parent.ActivateAbility` Instigator)
  (bind _ascharacter (cast `Character` Instigator))
  (bind _output_get (set `self.Character` _ascharacter))
  (`Character.Jump` _output_get)
  (add `Character.LandedDelegate` _output_get (`|CreateDelegate` :!event `LandedDelegate_Event`)))

(event `self.EndAbility`
  (params (Instigator :type "Actor Object Reference"))
  (`parent.EndAbility` Instigator)
  (remove `Character.LandedDelegate` (`self.Character`) (delegate `LandedDelegate_Event`)))

(event `LandedDelegate_Event`
  (params (Hit :type "HitResult Structure (by ref)"))
  (`self.EndAbility` (`self.Character`)))